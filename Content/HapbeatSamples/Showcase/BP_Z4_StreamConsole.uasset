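; BP_Z4_StreamConsole is a Hapbeat showcase zone actor that demonstrates a haptic loop with live gain and pan control.
; The construction script points the gain and pan bindings at LoopTrigger, and Space toggles that trigger between fire and stop.
; Zone activation seeds both bindings, creates the slider console widget with a tick trigger and sound, and shows the address panel.
; Deactivation stops the loop, removes the console and hides the panel.
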(event `Key|SpaceBar`
  (params (Key :type "Key Structure"))
  (bind _returnvalue (`HapbeatTriggerComponent.GetActivePlayback` (`self.LoopTrigger`)))
  ;[0.18 0.18 0.18] SPACE  |  live or Deferred loop: Stop  |  otherwise: Fire
  (:`Pressed`
    (if (`KismetSystemLibrary.IsValid` _returnvalue)
      (if (`HapbeatStreamPlayback.IsStopped` _returnvalue)
        ;[0.1 0.42 0.22] ON SHOWCASE ZONE ACTIVATED  |  seed bindings, create console, show address override
        (`HapbeatTriggerComponent.Fire` (`self.LoopTrigger`) :!label _label)
        (else
          (`HapbeatTriggerComponent.Stop` (`self.LoopTrigger`))))
      (else
        (goto _label)))))

(event `self.ReceiveZoneActivated`
  ;[0.1 0.42 0.22] ON SHOWCASE ZONE ACTIVATED  |  seed bindings, create console, show address override
  (`HapbeatParameterBinding.SetValue` (`self.GainBinding`) 0.5)
  (`HapbeatParameterBinding.SetValue` (`self.PanBinding`) 0.0)
  (bind _returnvalue (`WidgetBlueprintLibrary.Create` "/HapbeatSDK/HapbeatSamples/Showcase/BP_Z4_StreamConsoleWidget.BP_Z4_StreamConsoleWidget_C"))
  (bind _ashapbeat_showcase_z4console_widget (cast `HapbeatShowcaseZ4ConsoleWidget` _returnvalue))
  (`HapbeatShowcaseZ4ConsoleWidget.Configure` _ashapbeat_showcase_z4console_widget (`self.GainBinding`) (`self.PanBinding`) (`self.TickTrigger`) "/HapbeatSDK/HapbeatSamples/Showcase/Sounds/S_z4_ui_tick.S_z4_ui_tick")
  (`UserWidget.AddToViewport` _ashapbeat_showcase_z4console_widget 0)
  (set `self.ConsoleWidget` _ashapbeat_showcase_z4console_widget)
  (`HapbeatAddressOverridePanelComponent.Show` (`self.AddressPanel`)))

(event `self.ReceiveZoneDeactivated`
  (bind _consolewidget (`self.ConsoleWidget`))
  ;[0.5 0.15 0.15] ON SHOWCASE ZONE DEACTIVATED  |  stop loop, remove console, hide address override
  (`HapbeatTriggerComponent.Stop` (`self.LoopTrigger`))
  (if (`KismetSystemLibrary.IsValid` _consolewidget)
    (`UserWidget.RemoveFromParent` _consolewidget))
  (`HapbeatAddressOverridePanelComponent.Hide` (`self.AddressPanel`)))

(fn `UserConstructionScript`
  ;[0.1 0.42 0.22] CONNECT SLIDER BINDINGS TO THIS ACTOR'S LOOP TRIGGER
  (set `HapbeatParameterBinding.TargetTrigger` (`self.LoopTrigger`) (`self.GainBinding`))
  (set `HapbeatParameterBinding.TargetTrigger` (`self.LoopTrigger`) (`self.PanBinding`)))